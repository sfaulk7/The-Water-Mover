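; A puzzle obstacle platform that moves a cube along a spline and pauses temporarily when hit.
; The TravelSpline timeline scales its alpha by spline length to set the cube's local location along the path.
; Hit sets a Stopped flag for 7.5 seconds.
; Tick polls that flag to stop or resume the timeline and swap between plain and pulsing hex-tile materials.
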(event EventBeginPlay
  (bind _alpha (Timeline|TravelSpline Play)
    (:Update
      (Transformation|SetRelativeLocationAndRotation (Variables|Default|GetCube) (.location (Spline|GetTransformatDistanceAlongSpline (Variables|Default|GetSpline) (Math|Float|Lerp 0.0 _alpha (Spline|GetSplineLength (Variables|Default|GetSpline))) "Local" false)) "0, 0, 0" false false))))

(event EventTick
  (params (DeltaSeconds :type Float%20%28single-precision%29))
  (bind _cube (Variables|Default|GetCube))
  (if (Variables|Default|GetStopped)
    (Rendering|Material|SetMaterial _cube 0 "/Game/StarterContent/Materials/M_Tech_Hex_Tile.M_Tech_Hex_Tile")
    (bind _alpha (Timeline|TravelSpline Stop)
      (:Update
        (Transformation|SetRelativeLocationAndRotation (Variables|Default|GetCube) (.location (Spline|GetTransformatDistanceAlongSpline (Variables|Default|GetSpline) (Math|Float|Lerp 0.0 _alpha (Spline|GetSplineLength (Variables|Default|GetSpline))) "Local" false)) "0, 0, 0" false false)))
    (else
      (Rendering|Material|SetMaterial _cube 0 "/Game/StarterContent/Materials/M_Tech_Hex_Tile_Pulse.M_Tech_Hex_Tile_Pulse")
      (Timeline|TravelSpline Play))))

(event Collision|EventHit
  (params (MyComp :type Primitive%20Component%20Object%20Reference) (Other :type Actor%20Object%20Reference) (OtherComp :type Primitive%20Component%20Object%20Reference) (bSelfMoved :type Boolean) (HitLocation :type Vector :default "0, 0, 0") (HitNormal :type Vector :default "0, 0, 0") (NormalImpulse :type Vector :default "0, 0, 0") (Hit :type Hit%20Result%20Structure%20%28by%20ref%29))
  (Variables|Default|SetStopped true)
  (Utilities|FlowControl|Delay 7.5)
  (Variables|Default|SetStopped false))

(fn ConstructionScript)