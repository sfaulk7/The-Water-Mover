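; BP_WeightedCube is a puzzle cube that the player carries by holding the interact input.
; Any actor overlap toggles a pickup-range flag, while Tick casts the player character for the carry logic.
; While interact triggers in range or already carried, gravity is off and the cube sweeps to a point ahead of the character's WaterShootPoint along camera forward, with zeroed rotation.
; Releasing interact clears the carried state and restores gravity.
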(event Input|EnhancedActionEvents|EnhancedInputActionIA_Interact
  (params (ActionValue :type Boolean) (ElapsedSeconds :type Float%20%28double-precision%29) (TriggeredSeconds :type Float%20%28double-precision%29) (InputAction :type Input%20Action%20Object%20Reference :default "/Game/ThirdPerson/Input/Actions/IA_Interact.IA_Interact"))
  (bind _cube (Variables|Default|GetCube))
  (:Triggered
    (if (or (Variables|Default|GetWithinPickupRange) (Variables|Default|GetBeingCarried))
      (Variables|Default|SetBeingCarried true)
      (Physics|SetEnableGravity _cube false)
      (Transformation|SetWorldLocation _cube (+ (Transformation|GetWorldLocation (Variables|/Game/ThirdPerson/Blueprints/BP_ThirdPersonCharacter.BP_ThirdPersonCharacter_C|GetWaterShootPoint (stale EventTick _asbp_third_person_character))) (* (Math|Vector|GetForwardVector (Variables|/Script/Engine.PlayerCameraManager|GetTransformComponent (Game|GetPlayerCameraManager 0))) "50.000000,50.000000,50.000000")) true false)
      (Transformation|SetWorldRotation _cube "0, 0, 0" false false)))
  (:Completed
    (Variables|Default|SetBeingCarried false)
    (Physics|SetEnableGravity _cube true)))

(event Collision|EventActorBeginOverlap
  (params (OtherActor :type Actor%20Object%20Reference))
  (Variables|Default|SetWithinPickupRange true))

(event Collision|EventActorEndOverlap
  (params (OtherActor :type Actor%20Object%20Reference))
  (Variables|Default|SetWithinPickupRange false))

(event EventTick
  (params (DeltaSeconds :type Float%20%28single-precision%29))
  (bind _asbp_third_person_character (Utilities|Casting|CastToBP_ThirdPersonCharacter (Game|GetPlayerCharacter 0))))

(event EventBeginPlay
  (Input|EnableInput (Game|GetPlayerController 0)))

(fn ConstructionScript)