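; BP_IceContainer is a puzzle obstacle whose ice cube shrinks away while a linked pressure plate is weighed down.
; Tick polls the plate's WeighedDown flag and uses a short Delay to pace the shrinking into timed steps.
; Each step subtracts a fixed amount from the cube's world scale, and the whole actor is destroyed once the Z scale reaches zero or below.
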(event EventBeginPlay)

(event EventTick
  (params (DeltaSeconds :type Float%20%28single-precision%29))
  (bind _icecube (Variables|Default|GetIceCube))
  (bind _returnvalue (Transformation|GetWorldScale _icecube))
  (if (Variables|/Game/UnityCourse/Blueprint/Obstacles/Puzzle/BP_PressurePlate.BP_PressurePlate_C|GetWeighedDown (Variables|Default|GetPressurePlateRef))
    (Utilities|FlowControl|Delay 0.2)
    (Transformation|SetWorldScale3D _icecube (- (Math|Vector|MakeVector (.x _returnvalue) (.y _returnvalue) (.z _returnvalue)) "10.000000,10.000000,10.000000"))
    (if (<= (.z _returnvalue) 0.0)
      (Actor|DestroyActor))))

(fn ConstructionScript)