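; Puzzle obstacle with two sliding doors that respond to the weighed-down state of a referenced pressure plate.
; EffectDoors plays a Timeline that lerps both doors between closed and open world locations while the plate is pressed, and reverses it otherwise.
; Door positions are mirrored world-X offsets from Center, based on the root's X scale set at BeginPlay.
; Doors move with sweep, and a Hit event also reverses the Timeline.
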(event Custom|EffectDoors
  (bind (_closed _open) (|LeftDoorMovement))
  (bind (_closed_2 _open_2) (|RightDoorMovement))
  (if (Variables|/Game/UnityCourse/Blueprint/Obstacles/Puzzle/BP_PlayerPressurePlate.BP_PlayerPressurePlate_C|GetWeighedDown (Variables|Default|GetPressurePlateRef))
    (bind _alpha (Timeline|Timeline Play)
      (:Update
        (Transformation|SetWorldLocation (Variables|Default|GetLeftDoor) (Math|Vector|Lerp(Vector) _closed _open _alpha) true false)
        (Transformation|SetWorldLocation (Variables|Default|GetRightDoor) (Math|Vector|Lerp(Vector) _closed_2 _open_2 _alpha) true false)))
    (else
      (Timeline|Timeline Reverse))))

(event Custom|AfterColliison
  (bind (_closed _open) (|LeftDoorMovement))
  (bind (_closed_2 _open_2) (|RightDoorMovement))
  (bind _alpha (Timeline|Timeline Reverse)
    (:Update
      (Transformation|SetWorldLocation (Variables|Default|GetLeftDoor) (Math|Vector|Lerp(Vector) _closed _open _alpha) true false)
      (Transformation|SetWorldLocation (Variables|Default|GetRightDoor) (Math|Vector|Lerp(Vector) _closed_2 _open_2 _alpha) true false))))

(event EventBeginPlay
  (Variables|Default|SetMovementAmount (Math|Vector|MakeVector (Math|Conversions|ToFloat(Integer) (* (Math|Float|Truncate (.x (Transformation|GetWorldScale (Variables|Default|GetDefaultSceneRoot)))) 50)) 0.0 0.0)))

(event Collision|EventHit
  (params (MyComp :type Primitive%20Component%20Object%20Reference) (Other :type Actor%20Object%20Reference) (OtherComp :type Primitive%20Component%20Object%20Reference) (bSelfMoved :type Boolean) (HitLocation :type Vector :default "0, 0, 0") (HitNormal :type Vector :default "0, 0, 0") (NormalImpulse :type Vector :default "0, 0, 0") (Hit :type Hit%20Result%20Structure%20%28by%20ref%29))
  (CallFunction|AfterColliison))

(fn ConstructionScript)