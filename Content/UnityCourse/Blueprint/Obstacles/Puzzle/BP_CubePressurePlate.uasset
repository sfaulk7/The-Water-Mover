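; Pressure plate puzzle obstacle that responds to a BP Weighted Cube, identified by class display name on overlap.
; Begin overlap sets WeighedDown and lowers the Cube component in small delayed steps, counted by WhileCount.
; Tick mirrors WeighedDown onto the active state of WeighedCollision.
; End overlap clears WeighedDown before checking it, so the matching raise loop does not start as wired.
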(event Collision|EventActorBeginOverlap
  (params (OtherActor :type Actor%20Object%20Reference))
  (bind _cube (Variables|Default|GetCube))
  (bind _returnvalue (Transformation|GetWorldLocation _cube))
  (switch string (Utilities|GetClassDisplayName (Utilities|GetClass OtherActor))
    (:BP_WeightedCube_C
      (Variables|Default|SetWeighedDown true)
      ;[1 1 1] Moves the plate up and down
      (if (Variables|Default|GetWeighedDown) :!label _label
        (Transformation|SetWorldLocation _cube (Math|Vector|MakeVector (.x _returnvalue) (.y _returnvalue) (- (.z _returnvalue) 2.0)) false false)
        (Utilities|FlowControl|Delay 0.2)
        (Variables|Default|SetWhileCount (- (Variables|Default|GetWhileCount) 1))
        (if (>= (Variables|Default|GetWhileCount) 1)
          (goto _label))))))

(event Collision|EventActorEndOverlap
  (params (OtherActor :type Actor%20Object%20Reference))
  (bind _cube (Variables|Default|GetCube))
  (bind _returnvalue (Transformation|GetWorldLocation _cube))
  (switch string (Utilities|GetClassDisplayName (Utilities|GetClass OtherActor))
    (:BP_WeightedCube_C
      (Variables|Default|SetWeighedDown false)
      ;[1 1 1] Moves the plate up and down
      (if (Variables|Default|GetWeighedDown) :!label _label
        (Transformation|SetWorldLocation _cube (Math|Vector|MakeVector (.x _returnvalue) (.y _returnvalue) (+ (.z _returnvalue) 2.0)) false false)
        (Utilities|FlowControl|Delay 0.2)
        (Variables|Default|SetWhileCount (+ (Variables|Default|GetWhileCount) 1))
        (if (<= (Variables|Default|GetWhileCount) 9)
          (goto _label))))))

(event EventTick
  (params (DeltaSeconds :type Float%20%28single-precision%29))
  (bind _weighedcollision (Variables|Default|GetWeighedCollision))
  (if (Variables|Default|GetWeighedDown)
    (Components|Activation|SetActive _weighedcollision true false)
    (else
      (Components|Activation|SetActive _weighedcollision false false))))

(fn ConstructionScript)