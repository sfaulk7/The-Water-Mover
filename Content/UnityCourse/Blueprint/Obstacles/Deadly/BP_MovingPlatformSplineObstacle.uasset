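; Deadly moving platform obstacle that carries a cube along a spline, with a flame effect tied to its kill component.
; On BeginPlay the TravelSpline timeline scales its alpha by spline length and sets the cube's relative location to that point on the spline.
; Each Tick polls the BPCKill Inactive flag to switch the flames off when inactive and on otherwise.
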(event EventBeginPlay
  (bind _alpha (Timeline|TravelSpline Play)
    (:Update
      (Transformation|SetRelativeLocationAndRotation (Variables|Default|GetCube) (.location (Spline|GetTransformatDistanceAlongSpline (Variables|Default|GetSpline) (Math|Float|Lerp 0.0 _alpha (Spline|GetSplineLength (Variables|Default|GetSpline))) "Local" false)) "0, 0, 0" false false))))

(event EventTick
  (params (DeltaSeconds :type Float%20%28single-precision%29))
  (if (Variables|/Game/UnityCourse/Blueprint/Systems/BPC_Kill.BPC_Kill_C|GetInactive (Variables|Default|GetBPC_Kill))
    (Components|Activation|Deactivate (Variables|Default|GetFlames))
    (else
      (Components|Activation|Activate (Variables|Default|GetFlames) false))))

(fn ConstructionScript)