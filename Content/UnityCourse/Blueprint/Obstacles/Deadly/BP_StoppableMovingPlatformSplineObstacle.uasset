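; A deadly obstacle whose Cube travels along a spline and can be halted.
; The TravelSpline timeline scales its alpha by the spline length to set the Cube's local location, using only the location from the spline.
; Every Tick polls the BPCKill component's Inactive flag, stopping the timeline with a cooled lava material when inactive, otherwise playing it with the hot lava material.
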(event EventBeginPlay
  (bind _alpha (Timeline|TravelSpline Play)
    (:Update
      (Transformation|SetRelativeLocationAndRotation (Variables|Default|GetCube) (.location (Spline|GetTransformatDistanceAlongSpline (Variables|Default|GetSpline) (Math|Float|Lerp 0.0 _alpha (Spline|GetSplineLength (Variables|Default|GetSpline))) "Local" false)) "0, 0, 0" false false))))

(event EventTick
  (params (DeltaSeconds :type Float%20%28single-precision%29))
  (bind _cube (Variables|Default|GetCube))
  (if (Variables|/Game/UnityCourse/Blueprint/Systems/BPC_Kill.BPC_Kill_C|GetInactive (Variables|Default|GetBPC_Kill))
    (Rendering|Material|SetMaterial _cube 0 "/Game/UnityCourse/Blueprint/Materials/LavaMat/Materials/MI_LavaMat_10_Cooled.MI_LavaMat_10_Cooled")
    (bind _alpha (Timeline|TravelSpline Stop)
      (:Update
        (Transformation|SetRelativeLocationAndRotation (Variables|Default|GetCube) (.location (Spline|GetTransformatDistanceAlongSpline (Variables|Default|GetSpline) (Math|Float|Lerp 0.0 _alpha (Spline|GetSplineLength (Variables|Default|GetSpline))) "Local" false)) "0, 0, 0" false false)))
    (else
      (Rendering|Material|SetMaterial _cube 0 "/Game/UnityCourse/Blueprint/Materials/LavaMat/Materials/MI_LavaMat_10.MI_LavaMat_10")
      (Timeline|TravelSpline Play))))

(fn ConstructionScript)