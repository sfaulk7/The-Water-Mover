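; BP_SpinnerObstacle is a spinning obstacle that can be stopped, with a frozen effect, and restarted.
; Stop deactivates its RotatingMovement and reveals the FrozenSpiral effect, while Start resets and hides that effect and resumes rotation.
; The construction script gives the Cube a dynamic material with configurable base color and emission brightness.
; UpdateDynamicMaterial only casts materials on tagged meshes, without changing them.
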(event EventBeginPlay
  (Components|Activation|Activate (Variables|Default|GetFrozenSpiral) false)
  (Class|NiagaraComponent|SetPaused (Variables|Default|GetFrozenSpiral) true)
  (Development|SetHiddeninGame (Variables|Default|GetFrozenSpiral) true false))

(event EventUpdateDynamicMaterial
  (for _array_element (Actor|GetComponentsbyTag "/Script/Engine.StaticMeshComponent" "DynamicMaterial")
    (Utilities|Casting|CastToMaterialInstanceDynamic (Rendering|Material|GetMaterial _array_element 0))))

(event EventStart
  (bind _frozenspiral (Variables|Default|GetFrozenSpiral))
  (Class|NiagaraComponent|ClearSimCache _frozenspiral true)
  (Niagara|ResetSystem _frozenspiral)
  (Development|SetHiddeninGame _frozenspiral true false)
  (Class|NiagaraComponent|SetPaused _frozenspiral true)
  (Components|Activation|Activate (Variables|Default|GetRotatingMovement) false))

(event EventStop
  (bind _frozenspiral (Variables|Default|GetFrozenSpiral))
  (Development|SetHiddeninGame _frozenspiral false false)
  (Class|NiagaraComponent|SetPaused _frozenspiral false)
  (Components|Activation|Deactivate (Variables|Default|GetRotatingMovement)))

(fn ConstructionScript
  (bind _returnvalue (Rendering|Material|CreateDynamicMaterialInstance (Rendering|Material|GetMaterial (Variables|Default|GetCube) 0) "None" "None" :!class /Script/Engine.KismetMaterialLibrary))
  (Rendering|Material|SetVectorParameterValue _returnvalue "Base Color" (Variables|Default|GetBaseColor) :!class /Script/Engine.MaterialInstanceDynamic)
  (Rendering|Material|SetScalarParameterValue _returnvalue "EmissionBrightness" (Variables|Default|GetEmissionBrightness) :!class /Script/Engine.MaterialInstanceDynamic)
  (Rendering|Material|SetMaterial (Variables|Default|GetCube) 0 _returnvalue))