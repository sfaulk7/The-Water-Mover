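; BP_IcePowerUp is a collectable that unlocks the player's freeze ability when picked up.
; The construction script gives its InterpToMovement component relative StartPos and EndPos control points, defining a movement path.
; On overlap, it matches the other actor's class display name against the third-person character, calls UnlockFreeze on the first player controller's BP_PlayerState, then destroys itself.
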(event Collision|EventActorBeginOverlap
  (params (OtherActor :type Actor%20Object%20Reference))
  (switch string (Utilities|GetClassDisplayName (Utilities|GetClass OtherActor))
    (:BP_ThirdPersonCharacter_C
      (bind _asbp_player_state (Utilities|Casting|CastToBP_PlayerState (Variables|/Script/Engine.Controller|GetPlayerState (Game|GetPlayerController 0))))
      (Default|UnlockFreeze _asbp_player_state)
      (Actor|DestroyActor))))

(fn ConstructionScript
  (bind _interptomovement (Variables|Default|GetInterpToMovement))
  (Class|InterptoMovementComponent|AddControlPointPosition _interptomovement (Variables|Default|GetStartPos) true)
  (Class|InterptoMovementComponent|AddControlPointPosition _interptomovement (Variables|Default|GetEndPos) true))