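; Player state Blueprint that tracks collected coins, a water amount and whether the freeze ability is unlocked.
; Update functions change coins and water, with water clamped to a small fixed range, then broadcast the new values through coin and water update dispatchers.
; UpdateCoins returns the stored total plus the added coins again, so its return value differs from the broadcast one.
; UnlockFreeze simply sets its flag, without a broadcast.
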(event Custom|CustomEvent)

(event EventBeginPlay)

(event EventTick
  (params (DeltaSeconds :type Float%20%28single-precision%29)))

(fn ConstructionScript)

(fn UpdateCoins
  (params (Add%20Coins :type Integer))
  (bind _output_get (Variables|Default|SetCoinsCollected (+ (Variables|Default|GetCoinsCollected) Add%20Coins)))
  (Default|CallOnCoinUpdate _output_get)
  (return (+ (Variables|Default|GetCoinsCollected) Add%20Coins)))

(fn UpdateWaterAmount
  (params (Update%20Water :type Integer))
  (bind _output_get (Variables|Default|SetWaterAmount (Math|Integer|Clamp(Integer) (+ Update%20Water (Variables|Default|GetWaterAmount)) 0 3)))
  (Default|CallOnWaterUpdate _output_get)
  (Development|PrintString (Utilities|String|ToString(Integer) _output_get))
  (return _output_get))

(fn UnlockFreeze
  (bind _output_get (Variables|Default|SetFreezeUnlocked true))
  (return _output_get))