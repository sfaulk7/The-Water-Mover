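; BP_WaterPool is an interactable water pool that updates the player's water amount when used nearby.
; It enables input at start and tracks proximity through actor overlaps, matching the third-person character by class display name and printing the flag.
; When IA_Interact starts while the player is near, it casts player 0's PlayerState to BP_PlayerState and calls UpdateWaterAmount with 1.
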(event Input|EnhancedActionEvents|EnhancedInputActionIA_Interact
  (params (ActionValue :type Boolean) (ElapsedSeconds :type Float%20%28double-precision%29) (TriggeredSeconds :type Float%20%28double-precision%29) (InputAction :type Input%20Action%20Object%20Reference :default "/Game/ThirdPerson/Input/Actions/IA_Interact.IA_Interact"))
  (:Started
    (if (Variables|Default|GetPlayerNearby)
      (bind _asbp_player_state (Utilities|Casting|CastToBP_PlayerState (Variables|/Script/Engine.Controller|GetPlayerState (Game|GetPlayerController 0))))
      (Default|UpdateWaterAmount _asbp_player_state 1))))

(event Collision|EventActorBeginOverlap
  (params (OtherActor :type Actor%20Object%20Reference))
  (switch string (Utilities|GetClassDisplayName (Utilities|GetClass OtherActor))
    (:BP_ThirdPersonCharacter_C
      (Variables|Default|SetPlayerNearby true)
      (Development|PrintString (Utilities|String|ToString(Boolean) (Variables|Default|GetPlayerNearby))))))

(event Collision|EventActorEndOverlap
  (params (OtherActor :type Actor%20Object%20Reference))
  (switch string (Utilities|GetClassDisplayName (Utilities|GetClass OtherActor))
    (:BP_ThirdPersonCharacter_C
      (Variables|Default|SetPlayerNearby false)
      (Development|PrintString (Utilities|String|ToString(Boolean) (Variables|Default|GetPlayerNearby))))))

(event EventBeginPlay
  (Input|EnableInput (Game|GetPlayerController 0)))

(fn ConstructionScript)