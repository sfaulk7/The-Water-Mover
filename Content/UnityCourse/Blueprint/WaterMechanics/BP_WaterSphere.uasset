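; BP_WaterSphere is a water sphere actor that plays a burst effect from spawn and splashes on collision or after a short timeout.
; A sphere hit, bound every Tick, or the BeginPlay delay runs a one-time sequence guarded by Cleared.
; That sequence detaches and stops the burst, hides the sphere, disables its collision, plays the splash, then destroys the actor after delays.
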(event Custom|OnCollision
  (params (HitComponent :type Primitive%20Component%20Object%20Reference) (OtherActor :type Actor%20Object%20Reference) (OtherComp :type Primitive%20Component%20Object%20Reference) (NormalImpulse :type Vector) (Hit :type Hit%20Result%20Structure%20%28by%20ref%29))
  (bind _waterburst_system (Variables|Default|GetWaterBurst_System))
  (bind _sphere (Variables|Default|GetSphere))
  (bind _watersplash_system (Variables|Default|GetWaterSplash_System))
  (if (not (Variables|Default|GetCleared))
    (Transformation|DetachFromComponent _waterburst_system "KeepRelative" "KeepRelative" "KeepRelative" true)
    (Development|SetHiddeninGame _sphere true false)
    (Collision|SetCollisionEnabled _sphere "NoCollision")
    (Components|Activation|Deactivate _waterburst_system)
    (if (Components|Activation|IsActive _watersplash_system)
      _
      (else
        (Components|Activation|Activate _watersplash_system false)))
    (Variables|Default|SetCleared true)
    (Utilities|FlowControl|Delay 2.5)
    (Components|Activation|Deactivate _watersplash_system)
    (Utilities|FlowControl|Delay 2.0)
    (Actor|DestroyActor)))

(event EventBeginPlay
  (bind _waterburst_system (Variables|Default|GetWaterBurst_System))
  (bind _sphere (Variables|Default|GetSphere))
  (bind _watersplash_system (Variables|Default|GetWaterSplash_System))
  (Components|Activation|Activate _waterburst_system false)
  (Utilities|FlowControl|Delay 2.5)
  (if (not (Variables|Default|GetCleared))
    (Transformation|DetachFromComponent _waterburst_system "KeepRelative" "KeepRelative" "KeepRelative" true)
    (Development|SetHiddeninGame _sphere true false)
    (Collision|SetCollisionEnabled _sphere "NoCollision")
    (Components|Activation|Deactivate _waterburst_system)
    (if (Components|Activation|IsActive _watersplash_system)
      _
      (else
        (Components|Activation|Activate _watersplash_system false)))
    (Variables|Default|SetCleared true)
    (Utilities|FlowControl|Delay 2.5)
    (Components|Activation|Deactivate _watersplash_system)
    (Utilities|FlowControl|Delay 2.0)
    (Actor|DestroyActor)))

(event EventTick
  (params (DeltaSeconds :type Float%20%28single-precision%29))
  (Collision|BindEventtoOnComponentHit (Variables|Default|GetSphere) (delegate Custom|OnCollision)))

(fn ConstructionScript)