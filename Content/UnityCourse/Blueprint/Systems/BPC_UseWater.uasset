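; Player water-ability component that shoots water spheres or, once freeze is unlocked, places ice platforms, spending water per use.
; F toggles modes and HUD UI; holding right mouse aims, turning character and Aqua Crystal with the camera.
; While aiming, a delay loop predicts projectile paths and spawns trajectory markers or an ice preview at the path's end.
; Left click fires or places; mouse wheel and R adjust platform distance through simulation time.
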(event EventBeginPlay
  ;[1 1 1] Swaps UI between freeze UI and water UI
  (bind _aswater_hud (Utilities|Casting|CastToWaterHUD (HUD|GetHUD (Game|GetPlayerController 0))))
  (Default|SwapUI (Variables|/Game/Blueprints/WaterHUD.WaterHUD_C|GetUI%20Ref _aswater_hud) (Variables|Default|GetIsInFreezeMode))
  ;[1 1 1] Shooting out the water when left click is presses while aiming and not in freeze mode
  (bind _asbp_player_state (Utilities|Casting|CastToBP_PlayerState (Variables|/Script/Engine.Controller|GetPlayerState (Game|GetPlayerController 0)))))

(event EventTick
  (params (DeltaSeconds :type Float%20%28single-precision%29))
  (bind _returnvalue (Game|GetPlayerCameraManager 0))
  (bind _returnvalue_2 (Camera|GetCameraRotation _returnvalue))
  (bind _asbp_third_person_character (Utilities|Casting|CastToBP_ThirdPersonCharacter (Game|GetPlayerCharacter 0)))
  ;[1 1 1] Aqua Crystal and Player rotation while aiming
  (if (== (Variables|/Game/ThirdPerson/Blueprints/BP_ThirdPersonCharacter.BP_ThirdPersonCharacter_C|GetAiming _asbp_third_person_character) true)
    (Transformation|SetActorRotation _asbp_third_person_character (Math|Rotator|MakeRotator 0.0 0.0 (.yaw (Camera|GetCameraRotation (Game|GetPlayerCameraManager 0)))))
    (Transformation|SetWorldRotation (Variables|/Game/ThirdPerson/Blueprints/BP_ThirdPersonCharacter.BP_ThirdPersonCharacter_C|GetAquaCrystal _asbp_third_person_character) (Math|Rotator|MakeRotator (.roll _returnvalue_2) (+ (.pitch _returnvalue_2) -9e+01) (.yaw _returnvalue_2)) false false)))

(event Input|MouseEvents|LeftMouseButton
  (params (Key :type Key%20Structure :default "None"))
  (bind _returnvalue (Game|GetPlayerCameraManager 0))
  (bind _transformcomponent (Variables|/Script/Engine.PlayerCameraManager|GetTransformComponent _returnvalue))
  (bind _returnvalue_2 (Math|Vector|GetForwardVector _transformcomponent))
  ;[1 1 1] Shooting out the water when left click is presses while aiming and not in freeze mode
  (:Pressed
    (if (Variables|/Game/ThirdPerson/Blueprints/BP_ThirdPersonCharacter.BP_ThirdPersonCharacter_C|GetAiming (stale EventTick _asbp_third_person_character))
      (if (Variables|Default|GetIsInFreezeMode)
        (if (Variables|/Game/UnityCourse/Blueprint/BP_PlayerState.BP_PlayerState_C|GetFreezeUnlocked (stale EventBeginPlay _asbp_player_state))
          ;[1 1 1] Spawns ice platform
          (bind _asbp_player_state (Utilities|Casting|CastToBP_PlayerState (Variables|/Script/Engine.Controller|GetPlayerState (Game|GetPlayerController 0))))
          (if (Math|Conversions|ToBoolean(Integer) (Variables|/Game/UnityCourse/Blueprint/BP_PlayerState.BP_PlayerState_C|GetWaterAmount _asbp_player_state))
            (Game|SpawnActorfromClass "/Game/UnityCourse/Blueprint/WaterMechanics/BP_FrozenPlatform.BP_FrozenPlatform_C" (Variables|Default|GetIcePlatformSpawningPosition) "AlwaysSpawn" "MultiplyWithRoot" 0 0)
            (Default|UpdateWaterAmount _asbp_player_state -1)))
        (elif (Math|Conversions|ToBoolean(Integer) (Variables|/Game/UnityCourse/Blueprint/BP_PlayerState.BP_PlayerState_C|GetWaterAmount (stale EventBeginPlay _asbp_player_state)))
          (bind _returnvalue_3 (Game|SpawnActorfromClass "/Game/UnityCourse/Blueprint/WaterMechanics/BP_WaterSphere.BP_WaterSphere_C" (Math|Conversions|ToTransform(Vector) (Transformation|GetWorldLocation (Variables|/Game/ThirdPerson/Blueprints/BP_ThirdPersonCharacter.BP_ThirdPersonCharacter_C|GetWaterShootPoint (stale EventTick _asbp_third_person_character)))) "AlwaysSpawn" "MultiplyWithRoot" 0 0))
          (Default|UpdateWaterAmount (stale EventBeginPlay _asbp_player_state) -1)
          (Physics|AddImpulse (Variables|/Game/UnityCourse/Blueprint/WaterMechanics/BP_WaterSphere.BP_WaterSphere_C|GetSphere _returnvalue_3) (* "1000.000000,1000.000000,1000.000000" (Math|Vector|MakeVector (.x _returnvalue_2) (.y _returnvalue_2) (.z _returnvalue_2))) "None" true))))))

(event Input|MouseEvents|RightMouseButton
  (params (Key :type Key%20Structure :default "None"))
  (bind _returnvalue (Game|GetPlayerCameraManager 0))
  (bind _returnvalue_2 (Game|GetPlayerCameraManager 0))
  (bind _transformcomponent (Variables|/Script/Engine.PlayerCameraManager|GetTransformComponent _returnvalue_2))
  (bind _transformcomponent_2 (Variables|/Script/Engine.PlayerCameraManager|GetTransformComponent _returnvalue))
  (bind _returnvalue_3 (Math|Vector|GetForwardVector _transformcomponent_2))
  (bind _returnvalue_4 (Math|Vector|GetForwardVector _transformcomponent))
  (:Pressed
    (Variables|/Game/ThirdPerson/Blueprints/BP_ThirdPersonCharacter.BP_ThirdPersonCharacter_C|SetAiming (stale EventTick _asbp_third_person_character) true)
    (if (Variables|/Game/ThirdPerson/Blueprints/BP_ThirdPersonCharacter.BP_ThirdPersonCharacter_C|GetAiming (stale EventTick _asbp_third_person_character))
      (if (Variables|Default|GetIsInFreezeMode)
        (if (Variables|/Game/UnityCourse/Blueprint/BP_PlayerState.BP_PlayerState_C|GetFreezeUnlocked (stale EventBeginPlay _asbp_player_state))
          ;[1 1 1] Show Spawning location of ice platform
          (bind _predictresult (Class|GameplayStatics|BlueprintPredictProjectilePathAdvanced (Utilities|Struct|MakePredictProjectilePathParams (Transformation|GetWorldLocation (Variables|/Game/ThirdPerson/Blueprints/BP_ThirdPersonCharacter.BP_ThirdPersonCharacter_C|GetWaterShootPoint (stale EventTick _asbp_third_person_character))) (* "10000.000000,10000.000000,10000.000000" (Math|Vector|MakeVector (.x _returnvalue_3) (.y _returnvalue_3) (.z _returnvalue_3))) true 0.0 (Variables|Default|GetSimTime) true "ECC_WorldStatic" "ObjectTypeQuery1" 0 1e+01 0.0 "None" 0.0 false) :!label _label))
          (for _array_element (.pathdata _predictresult)
            _)
          (bind _returnvalue_5 (Game|SpawnActorfromClass "/Game/UnityCourse/Blueprint/Particles/BP_IcePlacementVisual.BP_IcePlacementVisual_C" (Math|Transform|MakeTransform (.location _array_element) "0, 0, 0" "1.000000,1.000000,1.000000") "AlwaysSpawn" "MultiplyWithRoot" 0 0))
          (Variables|Default|SetIcePlatformSpawningPosition (Transformation|GetActorTransform _returnvalue_5))
          (Utilities|FlowControl|Delay 0.01)
          (if (== (Variables|/Game/ThirdPerson/Blueprints/BP_ThirdPersonCharacter.BP_ThirdPersonCharacter_C|GetAiming (stale EventTick _asbp_third_person_character)) true)
            (if (Variables|Default|GetIsInFreezeMode)
              (goto _label))))
        (else
          ;[1 1 1] Show trajectory path of water
          (bind _predictresult_2 (Class|GameplayStatics|BlueprintPredictProjectilePathAdvanced (Utilities|Struct|MakePredictProjectilePathParams (Transformation|GetWorldLocation (Variables|/Game/ThirdPerson/Blueprints/BP_ThirdPersonCharacter.BP_ThirdPersonCharacter_C|GetWaterShootPoint (stale EventTick _asbp_third_person_character))) (* "1000.000000,1000.000000,1000.000000" (Math|Vector|MakeVector (.x _returnvalue_4) (.y _returnvalue_4) (.z _returnvalue_4))) true 0.0 1.0 true "ECC_WorldStatic" "ObjectTypeQuery1" 0 1e+01 0.0 "None" 0.0 false) :!label _label_2))
          (for _array_element_2 (.pathdata _predictresult_2)
            (Game|SpawnActorfromClass "/Game/UnityCourse/Blueprint/Particles/BP_TrajectoryLIne.BP_TrajectoryLIne_C" (Math|Transform|MakeTransform (.location _array_element_2) (Math|Rotator|MakeRotfromZ (.velocity _array_element_2)) "1.000000,1.000000,1.000000") "AlwaysSpawn" "MultiplyWithRoot" 0 0))
          (Utilities|FlowControl|Delay 0.01)
          (if (== (Variables|/Game/ThirdPerson/Blueprints/BP_ThirdPersonCharacter.BP_ThirdPersonCharacter_C|GetAiming (stale EventTick _asbp_third_person_character)) true)
            (if (not (Variables|Default|GetIsInFreezeMode))
              (goto _label_2)))))))
  (:Released
    (Variables|/Game/ThirdPerson/Blueprints/BP_ThirdPersonCharacter.BP_ThirdPersonCharacter_C|SetAiming (stale EventTick _asbp_third_person_character) false)))

(event Input|KeyboardEvents|R
  (params (Key :type Key%20Structure :default "None"))
  ;[1 1 1] Manipulates sim time to alter how far the ice platform will spawn
  (:Pressed
    (Variables|Default|SetSimTime 0.05)))

(event Input|MouseEvents|MouseWheelUp
  (params (Key :type Key%20Structure :default "None"))
  ;[1 1 1] Manipulates sim time to alter how far the ice platform will spawn
  (:Pressed
    (Variables|Default|SetSimTime (+ (Variables|Default|GetSimTime) 0.01))))

(event Input|MouseEvents|MouseWheelDown
  (params (Key :type Key%20Structure :default "None"))
  ;[1 1 1] Manipulates sim time to alter how far the ice platform will spawn
  (:Pressed
    (if (> (Variables|Default|GetSimTime) 0.0)
      (Variables|Default|SetSimTime (- (Variables|Default|GetSimTime) 0.01)))))

(event Input|KeyboardEvents|F
  (params (Key :type Key%20Structure :default "None"))
  (bind _returnvalue (Game|GetPlayerCameraManager 0))
  (bind _returnvalue_2 (Game|GetPlayerCameraManager 0))
  (bind _transformcomponent (Variables|/Script/Engine.PlayerCameraManager|GetTransformComponent _returnvalue_2))
  (bind _transformcomponent_2 (Variables|/Script/Engine.PlayerCameraManager|GetTransformComponent _returnvalue))
  (bind _returnvalue_3 (Math|Vector|GetForwardVector _transformcomponent_2))
  (bind _returnvalue_4 (Math|Vector|GetForwardVector _transformcomponent))
  ;[1 1 1] Swapping between freeze mode
  (:Pressed
    (bind _asbp_player_state (Utilities|Casting|CastToBP_PlayerState (Variables|/Script/Engine.Controller|GetPlayerState (Game|GetPlayerController 0))))
    (if (Variables|/Game/UnityCourse/Blueprint/BP_PlayerState.BP_PlayerState_C|GetFreezeUnlocked _asbp_player_state)
      (Utilities|FlowControl|FlipFlop
        (:A
          (Variables|Default|SetIsInFreezeMode true))
        (:B
          (Variables|Default|SetIsInFreezeMode false)))
      ;[1 1 1] Swaps UI between freeze UI and water UI
      (Default|SwapUI (Variables|/Game/Blueprints/WaterHUD.WaterHUD_C|GetUI%20Ref (stale EventBeginPlay _aswater_hud)) (Variables|Default|GetIsInFreezeMode))
      (if (Variables|/Game/ThirdPerson/Blueprints/BP_ThirdPersonCharacter.BP_ThirdPersonCharacter_C|GetAiming (stale EventTick _asbp_third_person_character))
        (if (Variables|Default|GetIsInFreezeMode)
          (if (Variables|/Game/UnityCourse/Blueprint/BP_PlayerState.BP_PlayerState_C|GetFreezeUnlocked (stale EventBeginPlay _asbp_player_state))
            ;[1 1 1] Show Spawning location of ice platform
            (bind _predictresult (Class|GameplayStatics|BlueprintPredictProjectilePathAdvanced (Utilities|Struct|MakePredictProjectilePathParams (Transformation|GetWorldLocation (Variables|/Game/ThirdPerson/Blueprints/BP_ThirdPersonCharacter.BP_ThirdPersonCharacter_C|GetWaterShootPoint (stale EventTick _asbp_third_person_character))) (* "10000.000000,10000.000000,10000.000000" (Math|Vector|MakeVector (.x _returnvalue_3) (.y _returnvalue_3) (.z _returnvalue_3))) true 0.0 (Variables|Default|GetSimTime) true "ECC_WorldStatic" "ObjectTypeQuery1" 0 1e+01 0.0 "None" 0.0 false) :!label _label))
            (for _array_element (.pathdata _predictresult)
              _)
            (bind _returnvalue_5 (Game|SpawnActorfromClass "/Game/UnityCourse/Blueprint/Particles/BP_IcePlacementVisual.BP_IcePlacementVisual_C" (Math|Transform|MakeTransform (.location _array_element) "0, 0, 0" "1.000000,1.000000,1.000000") "AlwaysSpawn" "MultiplyWithRoot" 0 0))
            (Variables|Default|SetIcePlatformSpawningPosition (Transformation|GetActorTransform _returnvalue_5))
            (Utilities|FlowControl|Delay 0.01)
            (if (== (Variables|/Game/ThirdPerson/Blueprints/BP_ThirdPersonCharacter.BP_ThirdPersonCharacter_C|GetAiming (stale EventTick _asbp_third_person_character)) true)
              (if (Variables|Default|GetIsInFreezeMode)
                (goto _label))))
          (else
            ;[1 1 1] Show trajectory path of water
            (bind _predictresult_2 (Class|GameplayStatics|BlueprintPredictProjectilePathAdvanced (Utilities|Struct|MakePredictProjectilePathParams (Transformation|GetWorldLocation (Variables|/Game/ThirdPerson/Blueprints/BP_ThirdPersonCharacter.BP_ThirdPersonCharacter_C|GetWaterShootPoint (stale EventTick _asbp_third_person_character))) (* "1000.000000,1000.000000,1000.000000" (Math|Vector|MakeVector (.x _returnvalue_4) (.y _returnvalue_4) (.z _returnvalue_4))) true 0.0 1.0 true "ECC_WorldStatic" "ObjectTypeQuery1" 0 1e+01 0.0 "None" 0.0 false) :!label _label_2))
            (for _array_element_2 (.pathdata _predictresult_2)
              (Game|SpawnActorfromClass "/Game/UnityCourse/Blueprint/Particles/BP_TrajectoryLIne.BP_TrajectoryLIne_C" (Math|Transform|MakeTransform (.location _array_element_2) (Math|Rotator|MakeRotfromZ (.velocity _array_element_2)) "1.000000,1.000000,1.000000") "AlwaysSpawn" "MultiplyWithRoot" 0 0))
            (Utilities|FlowControl|Delay 0.01)
            (if (== (Variables|/Game/ThirdPerson/Blueprints/BP_ThirdPersonCharacter.BP_ThirdPersonCharacter_C|GetAiming (stale EventTick _asbp_third_person_character)) true)
              (if (not (Variables|Default|GetIsInFreezeMode))
                (goto _label_2)))))))))