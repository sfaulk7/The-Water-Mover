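; Actor component that turns its owner, such as a spinner, into a hot hazard that destroys the third-person character on contact.
; On BeginPlay it binds hit events on the owner's static meshes tagged "Kill", then branches on the other actor's class name.
; A water sphere hit clears IsHot and messages the owner to stop, then restores both after a delay.
; Tick messages the owner to update its dynamic material.
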(event Custom|OnHItKill
  (params (HitComponent :type Primitive%20Component%20Object%20Reference) (OtherActor :type Actor%20Object%20Reference) (OtherComp :type Primitive%20Component%20Object%20Reference) (NormalImpulse :type Vector) (Hit :type Hit%20Result%20Structure%20%28by%20ref%29))
  (bind _returnvalue (Components|GetOwner))
  ;[1 1 1] Kill Player when contacting a spinner
  (Development|PrintString "Hit")
  (switch string (Utilities|GetClassDisplayName (Utilities|GetClass OtherActor))
    (:BP_ThirdPersonCharacter_C
      (if (Variables|Default|GetIsHot)
        (Actor|DestroyActor OtherActor)))
    (:BP_WaterSphere_C
      (bind _output_get (Variables|Default|SetIsHot false))
      (Development|PrintString (Utilities|String|ToString(Boolean) _output_get))
      (Variables|Default|SetInactive true)
      (Class|BPIObstacle|Stop(Message) _returnvalue)
      (Utilities|FlowControl|Delay 7.5)
      (Class|BPIObstacle|Start(Message) _returnvalue)
      (bind _output_get_2 (Variables|Default|SetIsHot true))
      (Development|PrintString (Utilities|String|ToString(Boolean) _output_get_2))
      (Variables|Default|SetInactive false))))

(event EventTick
  (params (DeltaSeconds :type Float%20%28single-precision%29))
  ;[1 1 1] Kill Player when contacting a spinner
  (Class|BPIObstacle|UpdateDynamicMaterial(Message) (Components|GetOwner)))

(event EventBeginPlay
  ;[1 1 1] Kill Player when contacting a spinner
  (for _array_element (Actor|GetComponentsbyTag (Components|GetOwner) "/Script/Engine.StaticMeshComponent" "Kill")
    (Collision|BindEventtoOnComponentHit _array_element (delegate Custom|OnHItKill))))